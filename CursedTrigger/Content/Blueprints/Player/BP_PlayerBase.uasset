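; Base player character that handles Enhanced Input for moving, looking, jumping, crouching and walking in multiplayer.
; Crouch and walk apply locally and, on remote machines, also call server events that run the same function.
; Both add or remove entries in a MovementState array used as a stack, whose last entry sets crouch and max walk speed.
; Jump relies on the engine's built-in replication and fires only when not falling.
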(event Custom|Server_Crouch
  (params (bCrouch :type Boolean))
  (CallFunction|FCrouch bCrouch))

(event Custom|Server_Walk
  (params (bWalk :type Boolean))
  (CallFunction|FWalk bWalk))

(event Input|EnhancedActionEvents|EnhancedInputActionIA_Movement
  (params (ActionValue :type Vector%202D%20Structure) (ElapsedSeconds :type Float%20%28double-precision%29) (TriggeredSeconds :type Float%20%28double-precision%29) (InputAction :type Input%20Action%20Object%20Reference :default "/Game/Blueprints/Player/Input/IA_Movement.IA_Movement"))
  (:Triggered
    (Pawn|Input|AddMovementInput (Transformation|GetActorForwardVector) (.x ActionValue) false)
    (Pawn|Input|AddMovementInput (Transformation|GetActorRightVector) (.y ActionValue) false)))

(event Input|EnhancedActionEvents|EnhancedInputActionIA_Look
  (params (ActionValue :type Vector%202D%20Structure) (ElapsedSeconds :type Float%20%28double-precision%29) (TriggeredSeconds :type Float%20%28double-precision%29) (InputAction :type Input%20Action%20Object%20Reference :default "/Game/Blueprints/Player/Input/IA_Look.IA_Look"))
  (:Triggered
    (Pawn|Input|AddControllerYawInput (.x ActionValue))
    (Pawn|Input|AddControllerPitchInput (.y ActionValue))))

(event Input|EnhancedActionEvents|EnhancedInputActionIA_Crouch
  (params (ActionValue :type Boolean) (ElapsedSeconds :type Float%20%28double-precision%29) (TriggeredSeconds :type Float%20%28double-precision%29) (InputAction :type Input%20Action%20Object%20Reference :default "/Game/Blueprints/Player/Input/IA_Crouch.IA_Crouch"))
  (:Triggered
    (if ActionValue
      (CallFunction|FCrouch true)
      (else
        (CallFunction|FCrouch false)))))

(event Input|EnhancedActionEvents|EnhancedInputActionIA_Walk
  (params (ActionValue :type Boolean) (ElapsedSeconds :type Float%20%28double-precision%29) (TriggeredSeconds :type Float%20%28double-precision%29) (InputAction :type Input%20Action%20Object%20Reference :default "/Game/Blueprints/Player/Input/IA_Walk.IA_Walk"))
  (:Triggered
    (if ActionValue
      (CallFunction|FWalk true)
      (else
        (CallFunction|FWalk false)))))

(event Input|EnhancedActionEvents|EnhancedInputActionIA_Jump
  (params (ActionValue :type Boolean) (ElapsedSeconds :type Float%20%28double-precision%29) (TriggeredSeconds :type Float%20%28double-precision%29) (InputAction :type Input%20Action%20Object%20Reference :default "/Game/Blueprints/Player/Input/IA_Jump.IA_Jump"))
  (:Triggered
    (if (CallFunction|FIsNotJumping)
      ;[0.415 0.2753 1] Jump in unreal is already replicated and multiplayer ready
      (Character|Jump))))

(event EventBeginPlay
  (bind _playercontroller (Class|INTPlayerController|GetPlayerControllerRef(Message) (Pawn|GetController)))
  (Utilities|IsValid _playercontroller
    (:Is%20Valid
      (Input|AddMappingContext (PlayerController|LocalPlayerSubsystems|GetEnhancedInputLocalPlayerSubsystem _playercontroller) "/Game/Blueprints/Player/Input/IMC_Default.IMC_Default" 0 "(bIgnoreAllPressedKeysUntilRelease=True,bForceImmediately=False)"))))

(fn ConstructionScript)

(fn FCrouch
  (params (bCrouch :type Boolean))
  (bind _movementstate (Variables|Default|GetMovementState))
  (bind _output_get (LocalVariables|SetcrouchLocal bCrouch))
  (Networking|SwitchHasAuthority
    (:Authority
      _)
    (:Remote
      (CallFunction|ServerCrouch _output_get)))
  (if (LocalVariables|GetcrouchLocal)
    (Character|Crouch)
    (Utilities|Array|SetArrayElem _movementstate (+ (Utilities|Array|LastIndex _movementstate) 1) "NewEnumerator5" true)
    (CallFunction|FSetMovementSpeed)
    (else
      (Character|UnCrouch)
      (Utilities|Array|RemoveItem (Variables|Default|GetMovementState) "NewEnumerator5")
      (CallFunction|FSetMovementSpeed))))

(fn FWalk
  (params (bWalk :type Boolean))
  (bind _movementstate (Variables|Default|GetMovementState))
  (bind _output_get (LocalVariables|SetwalkLocal bWalk))
  (Networking|SwitchHasAuthority
    (:Authority
      _)
    (:Remote
      (CallFunction|ServerWalk _output_get)))
  (if (LocalVariables|GetwalkLocal)
    (Utilities|Array|SetArrayElem _movementstate (+ (Utilities|Array|LastIndex _movementstate) 1) "NewEnumerator4" true)
    (CallFunction|FSetMovementSpeed)
    (else
      (Utilities|Array|RemoveItem (Variables|Default|GetMovementState) "NewEnumerator4")
      (CallFunction|FSetMovementSpeed))))

(fn FIsNotJumping
  (return (not (AI|Components|NavMovement|IsFalling (Variables|Character|GetCharacterMovement)))))

(fn FSetMovementSpeed
  (bind _movementstate (Variables|Default|GetMovementState))
  (bind _movementstate_2 (Variables|Default|GetMovementState))
  (if (Utilities|Enum|Equal(Enum) (Utilities|Array|Get(acopy) _movementstate (Utilities|Array|LastIndex _movementstate)) "NewEnumerator5")
    (Character|Crouch)
    (else
      (Character|UnCrouch)))
  (Variables|/Script/Engine.CharacterMovementComponent|SetMaxWalkSpeed (Variables|Character|GetCharacterMovement) (Utilities|Select :Index (Utilities|Array|Get(acopy) _movementstate_2 (Utilities|Array|LastIndex _movementstate_2)) :NewEnumerator0 (Variables|Default|GetRunSpeed) :NewEnumerator4 (Variables|Default|GetWalkSpeed) :NewEnumerator5 (Variables|Default|GetCrouchSpeed))))

(fn GetPlayerBaseRef
  (return self))